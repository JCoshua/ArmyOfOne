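; Player pawn for a tile-based tactics game that snaps to the selected tile and highlights unit ranges.
; Right stick steps a clamped target distance, which Tick eases the camera boom toward.
; Movement range paints reachable tiles blue, with occupied and outlying attackable tiles red; attack range recolors only the unit's current tile, ending blue.
; D-pad and mouse clicks toggle cursor visibility and the UsingMouse flag.
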(event `self.ReceiveBeginPlay`
  (set `PlayerController.bShowMouseCursor` true (`GameplayStatics.GetPlayerController` 0)))

(event `self.ReceiveTick`
  (params (DeltaSeconds :type "Float (single-precision)"))
  (bind _targetcameradistance (`self.TargetCameraDistance`))
  (bind (_socketoffset_x _socketoffset_y _socketoffset_z) (`KismetMathLibrary.BreakVector` (`SpringArmComponent.SocketOffset` (`self.CameraBoom`))))
  (bind _returnvalue (`KismetMathLibrary.MakeVector` (* _targetcameradistance -1.0) 0.0 _targetcameradistance))
  (`|ExecutionSequence`
    (:`then_0`
      (`self.K2_SetActorLocation` (+ (`self.K2_GetActorLocation` (`self.SelectedTile`)) (0.0 0.0 5.1))))
    (:`then_1`
      (if (`KismetMathLibrary.NearlyEqual_FloatFloat` _socketoffset_z (`self.TargetCameraDistance`) 1.0)
        (`/Engine/EditorBlueprintResources/StandardMacros.DoOnce` false :!label _label
          (:`Completed`
            (set `SpringArmComponent.SocketOffset` _returnvalue (`self.CameraBoom`))))
        (else
          (set `SpringArmComponent.SocketOffset` (`KismetMathLibrary.VLerp` (`SpringArmComponent.SocketOffset` (`self.CameraBoom`)) _returnvalue 0.2) (`self.CameraBoom`))
          (goto _label :!via `Reset`))))))

(event `InputAxisKey|Gamepad_RightY`
  (params (AxisValue :type "Float (single-precision)"))
  (bind _returnvalue (- (`self.TargetCameraDistance`) 100.0))
  (bind _returnvalue_2 (+ (`self.TargetCameraDistance`) 100.0))
  (if (<= AxisValue -0.99)
    (if (>= _returnvalue (`self.MinCameraDistance`))
      (set `self.TargetCameraDistance` _returnvalue))
    (elif (>= AxisValue 0.99)
      (if (<= _returnvalue_2 (`self.MaxCameraDistance`))
        (set `self.TargetCameraDistance` _returnvalue_2)))))

(event `self.ShowMoveRange`
  (params (unit :type "UnitActor Object Reference"))
  (`self.ShowMovementRange` unit))

(event `self.ShowAttackRange`
  (params (unit :type "UnitActor Object Reference"))
  (bind _currenttile (`UnitActor.CurrentTile` unit))
  (bind _movementmesh (`MapTileActor.MovementMesh` _currenttile))
  (bind _movementmesh_2 (`MapTileActor.MovementMesh` _currenttile))
  (`/Engine/EditorBlueprintResources/StandardMacros.IsValid` unit
    (:`Is Valid`
      (`self.ClearMapRange`)
      (bind _returnvalue (`UnitActor.GetAttackableTiles` unit _currenttile))
      (for _ _returnvalue
        (`SceneComponent.SetVisibility` _movementmesh true false)
        (`PrimitiveComponent.SetMaterial` _movementmesh 0 "/Game/Materials/MovementIndicators/MI_MovementIndicator_Red.MI_MovementIndicator_Red"))
      (`SceneComponent.SetVisibility` _movementmesh_2 true false)
      (`PrimitiveComponent.SetMaterial` _movementmesh_2 0 "/Game/Materials/MovementIndicators/MI_MovementIndicator_Blue.MI_MovementIndicator_Blue"))))

(event `Key|Gamepad_DPad_Up` :paused true
  (params (Key :type "Key Structure"))
  (bind _returnvalue (`GameplayStatics.GetPlayerController` 0))
  (:`Pressed`
    (if (`PlayerController.bShowMouseCursor` _returnvalue) :!label _label_2
      (set `PlayerController.bShowMouseCursor` false _returnvalue)
      (set `self.UsingMouse` false))))

(event `Key|Gamepad_DPad_Left` :paused true
  (params (Key :type "Key Structure"))
  (:`Pressed`
    (goto _label_2)))

(event `Key|Gamepad_DPad_Right` :paused true
  (params (Key :type "Key Structure"))
  (:`Pressed`
    (goto _label_2)))

(event `Key|Gamepad_DPad_Down` :paused true
  (params (Key :type "Key Structure"))
  (:`Pressed`
    (goto _label_2)))

(event `Key|LeftMouseButton`
  (params (Key :type "Key Structure"))
  (bind _returnvalue (`GameplayStatics.GetPlayerController` 0))
  (:`Pressed`
    (if (not (`PlayerController.bShowMouseCursor` _returnvalue)) :!label _label_3
      (set `PlayerController.bShowMouseCursor` true _returnvalue)
      (set `self.UsingMouse` true))))

(event `Key|RightMouseButton`
  (params (Key :type "Key Structure"))
  (:`Pressed`
    (goto _label_3)))

(fn `ShowMovementRange`
  (params (Unit :type "UnitActor Object Reference"))
  (locals (L_Unit :type "UnitActor Object Reference"))
  (bind _output_get (set `local.L_Unit` Unit))
  (`/Engine/EditorBlueprintResources/StandardMacros.IsValid` _output_get
    (:`Is Valid`
      (`self.ClearMapRange`)
      (bind _returnvalue (`UnitActor.GetAllTilesInRange` (`local.L_Unit`)))
      (for _array_element _returnvalue
        (`|ExecutionSequence`
          (:`then_0`
            (bind _unit (`MapTileActor.Unit` _array_element)
              (:`then`
                (if (!= _unit (`local.L_Unit`))
                  (`PrimitiveComponent.SetMaterial` (`MapTileActor.MovementMesh` _array_element) 0 "/Game/Materials/MovementIndicators/MI_MovementIndicator_Red.MI_MovementIndicator_Red")
                  (else
                    (bind _movementmesh (`MapTileActor.MovementMesh` _array_element))
                    (`PrimitiveComponent.SetMaterial` _movementmesh 0 "/Game/Materials/MovementIndicators/MI_MovementIndicator_Blue.MI_MovementIndicator_Blue" :!label _label))))
              (:`else`
                (goto _label)))
            (`SceneComponent.SetVisibility` _movementmesh true false))
          (:`then_1`
            (bind _returnvalue_2 (`UnitActor.GetAttackableTiles` (`local.L_Unit`) _array_element))
            (for _array_element_2 _returnvalue_2
              (if (not (`KismetArrayLibrary.Array_Contains` _returnvalue _array_element_2))
                (bind _movementmesh_2 (`MapTileActor.MovementMesh` _array_element_2))
                (`SceneComponent.SetVisibility` _movementmesh_2 true false)
                (`PrimitiveComponent.SetMaterial` _movementmesh_2 0 "/Game/Materials/MovementIndicators/MI_MovementIndicator_Red.MI_MovementIndicator_Red")))))))))

(fn `UserConstructionScript`)
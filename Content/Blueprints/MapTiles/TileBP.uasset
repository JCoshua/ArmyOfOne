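; TileBP is a map tile actor with functions that grow a grid map by spawning Plains, Forest or Water neighbours on its four sides.
; Each function checks MapData for an empty cell, spawns a tile 100 units away, sets its indices and registers it.
; Only Top and Bottom variants pass MapData to the new tile.
; AddBottomWater spawns a ForestTile despite its name.
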(fn `Add Bottom (Forest)`
  (bind _returnvalue (`MapManager.GetTile` (`self.MapData`) (`self.HorizontalIndex`) (- (`self.VerticalIndex`) 1)))
  (`/Engine/EditorBlueprintResources/StandardMacros.IsValid` _returnvalue
    (:`Is Not Valid`
      (bind _returnvalue_2 (`|SpawnActorFromClass` "/Game/Blueprints/MapTiles/ForestTile.ForestTile_C" (`KismetMathLibrary.MakeTransform` (+ (`self.K2_GetActorLocation`) (-100.0 0.0 0.0))) "Undefined" "OverrideRootScale" null null))
      (`|ExecutionSequence`
        (:`then_0`
          (set `TileActor.HorizontalIndex` (`self.HorizontalIndex`) _returnvalue_2))
        (:`then_1`
          (set `TileActor.VerticalIndex` (- (`self.VerticalIndex`) 1) _returnvalue_2))
        (:`then_2`
          (bind _output_get (set `TileActor.MapData` (`self.MapData`) _returnvalue_2))
          (`MapManager.AddTileToGrid` _output_get _returnvalue_2))))))

(fn `Add Bottom (Plains)`
  (bind _returnvalue (`MapManager.GetTile` (`self.MapData`) (`self.HorizontalIndex`) (- (`self.VerticalIndex`) 1)))
  (`/Engine/EditorBlueprintResources/StandardMacros.IsValid` _returnvalue
    (:`Is Not Valid`
      (bind _returnvalue_2 (`|SpawnActorFromClass` "/Game/Blueprints/MapTiles/PlainsTile.PlainsTile_C" (`KismetMathLibrary.MakeTransform` (+ (`self.K2_GetActorLocation`) (-100.0 0.0 0.0))) "Undefined" "OverrideRootScale" null null))
      (`|ExecutionSequence`
        (:`then_0`
          (set `TileActor.HorizontalIndex` (`self.HorizontalIndex`) _returnvalue_2))
        (:`then_1`
          (set `TileActor.VerticalIndex` (- (`self.VerticalIndex`) 1) _returnvalue_2))
        (:`then_2`
          (bind _output_get (set `TileActor.MapData` (`self.MapData`) _returnvalue_2))
          (`MapManager.AddTileToGrid` _output_get _returnvalue_2))))))

(fn `Add Bottom (Water)`
  (bind _returnvalue (`MapManager.GetTile` (`self.MapData`) (`self.HorizontalIndex`) (- (`self.VerticalIndex`) 1)))
  (`/Engine/EditorBlueprintResources/StandardMacros.IsValid` _returnvalue
    (:`Is Not Valid`
      (bind _returnvalue_2 (`|SpawnActorFromClass` "/Game/Blueprints/MapTiles/ForestTile.ForestTile_C" (`KismetMathLibrary.MakeTransform` (+ (`self.K2_GetActorLocation`) (-100.0 0.0 0.0))) "Undefined" "OverrideRootScale" null null))
      (`|ExecutionSequence`
        (:`then_0`
          (set `TileActor.HorizontalIndex` (`self.HorizontalIndex`) _returnvalue_2))
        (:`then_1`
          (set `TileActor.VerticalIndex` (- (`self.VerticalIndex`) 1) _returnvalue_2))
        (:`then_2`
          (bind _output_get (set `TileActor.MapData` (`self.MapData`) _returnvalue_2))
          (`MapManager.AddTileToGrid` _output_get _returnvalue_2))))))

(fn `Add Left (Forest)`
  (bind _returnvalue (`MapManager.GetTile` (`self.MapData`) (- (`self.HorizontalIndex`) 1) (`self.VerticalIndex`)))
  (`/Engine/EditorBlueprintResources/StandardMacros.IsValid` _returnvalue
    (:`Is Not Valid`
      (bind _returnvalue_2 (`|SpawnActorFromClass` "/Game/Blueprints/MapTiles/ForestTile.ForestTile_C" (`KismetMathLibrary.MakeTransform` (+ (`self.K2_GetActorLocation`) (0.0 -100.0 0.0))) "Undefined" "OverrideRootScale" null null))
      (`|ExecutionSequence`
        (:`then_0`
          (set `TileActor.HorizontalIndex` (- (`self.HorizontalIndex`) 1) _returnvalue_2))
        (:`then_1`
          (set `TileActor.VerticalIndex` (`self.VerticalIndex`) _returnvalue_2))
        (:`then_2`
          (`MapManager.AddTileToGrid` (`self.MapData`) _returnvalue_2))))))

(fn `Add Left (Plains)`
  (bind _returnvalue (`MapManager.GetTile` (`self.MapData`) (- (`self.HorizontalIndex`) 1) (`self.VerticalIndex`)))
  (`/Engine/EditorBlueprintResources/StandardMacros.IsValid` _returnvalue
    (:`Is Not Valid`
      (bind _returnvalue_2 (`|SpawnActorFromClass` "/Game/Blueprints/MapTiles/PlainsTile.PlainsTile_C" (`KismetMathLibrary.MakeTransform` (+ (`self.K2_GetActorLocation`) (0.0 -100.0 0.0))) "Undefined" "OverrideRootScale" null null))
      (`|ExecutionSequence`
        (:`then_0`
          (set `TileActor.HorizontalIndex` (- (`self.HorizontalIndex`) 1) _returnvalue_2))
        (:`then_1`
          (set `TileActor.VerticalIndex` (`self.VerticalIndex`) _returnvalue_2))
        (:`then_2`
          (`MapManager.AddTileToGrid` (`self.MapData`) _returnvalue_2))))))

(fn `Add Left (Water)`
  (bind _returnvalue (`MapManager.GetTile` (`self.MapData`) (- (`self.HorizontalIndex`) 1) (`self.VerticalIndex`)))
  (`/Engine/EditorBlueprintResources/StandardMacros.IsValid` _returnvalue
    (:`Is Not Valid`
      (bind _returnvalue_2 (`|SpawnActorFromClass` "/Game/Blueprints/MapTiles/WaterTile.WaterTile_C" (`KismetMathLibrary.MakeTransform` (+ (`self.K2_GetActorLocation`) (0.0 -100.0 0.0))) "Undefined" "OverrideRootScale" null null))
      (`|ExecutionSequence`
        (:`then_0`
          (set `TileActor.HorizontalIndex` (- (`self.HorizontalIndex`) 1) _returnvalue_2))
        (:`then_1`
          (set `TileActor.VerticalIndex` (`self.VerticalIndex`) _returnvalue_2))
        (:`then_2`
          (`MapManager.AddTileToGrid` (`self.MapData`) _returnvalue_2))))))

(fn `Add Right (Forest)`
  (bind _returnvalue (`MapManager.GetTile` (`self.MapData`) (+ (`self.HorizontalIndex`) 1) (`self.VerticalIndex`)))
  (`/Engine/EditorBlueprintResources/StandardMacros.IsValid` _returnvalue
    (:`Is Not Valid`
      (bind _returnvalue_2 (`|SpawnActorFromClass` "/Game/Blueprints/MapTiles/ForestTile.ForestTile_C" (`KismetMathLibrary.MakeTransform` (+ (`self.K2_GetActorLocation`) (0.0 100.0 0.0))) "Undefined" "OverrideRootScale" null null))
      (`|ExecutionSequence`
        (:`then_0`
          (set `TileActor.HorizontalIndex` (+ (`self.HorizontalIndex`) 1) _returnvalue_2))
        (:`then_1`
          (set `TileActor.VerticalIndex` (`self.VerticalIndex`) _returnvalue_2))
        (:`then_2`
          (`MapManager.AddTileToGrid` (`self.MapData`) _returnvalue_2))))))

(fn `Add Right (Plains)`
  (bind _returnvalue (`MapManager.GetTile` (`self.MapData`) (+ (`self.HorizontalIndex`) 1) (`self.VerticalIndex`)))
  (`/Engine/EditorBlueprintResources/StandardMacros.IsValid` _returnvalue
    (:`Is Not Valid`
      (bind _returnvalue_2 (`|SpawnActorFromClass` "/Game/Blueprints/MapTiles/PlainsTile.PlainsTile_C" (`KismetMathLibrary.MakeTransform` (+ (`self.K2_GetActorLocation`) (0.0 100.0 0.0))) "Undefined" "OverrideRootScale" null null))
      (`|ExecutionSequence`
        (:`then_0`
          (set `TileActor.HorizontalIndex` (+ (`self.HorizontalIndex`) 1) _returnvalue_2))
        (:`then_1`
          (set `TileActor.VerticalIndex` (`self.VerticalIndex`) _returnvalue_2))
        (:`then_2`
          (`MapManager.AddTileToGrid` (`self.MapData`) _returnvalue_2))))))

(fn `Add Right (Water)`
  (bind _returnvalue (`MapManager.GetTile` (`self.MapData`) (+ (`self.HorizontalIndex`) 1) (`self.VerticalIndex`)))
  (`/Engine/EditorBlueprintResources/StandardMacros.IsValid` _returnvalue
    (:`Is Not Valid`
      (bind _returnvalue_2 (`|SpawnActorFromClass` "/Game/Blueprints/MapTiles/WaterTile.WaterTile_C" (`KismetMathLibrary.MakeTransform` (+ (`self.K2_GetActorLocation`) (0.0 100.0 0.0))) "Undefined" "OverrideRootScale" null null))
      (`|ExecutionSequence`
        (:`then_0`
          (set `TileActor.HorizontalIndex` (+ (`self.HorizontalIndex`) 1) _returnvalue_2))
        (:`then_1`
          (set `TileActor.VerticalIndex` (`self.VerticalIndex`) _returnvalue_2))
        (:`then_2`
          (`MapManager.AddTileToGrid` (`self.MapData`) _returnvalue_2))))))

(fn `Add Top (Forest)`
  (bind _returnvalue (`MapManager.GetTile` (`self.MapData`) (`self.HorizontalIndex`) (+ (`self.VerticalIndex`) 1)))
  (`/Engine/EditorBlueprintResources/StandardMacros.IsValid` _returnvalue
    (:`Is Not Valid`
      (bind _returnvalue_2 (`|SpawnActorFromClass` "/Game/Blueprints/MapTiles/ForestTile.ForestTile_C" (`KismetMathLibrary.MakeTransform` (+ (`self.K2_GetActorLocation`) (100.0 0.0 0.0))) "Undefined" "OverrideRootScale" null null))
      (`|ExecutionSequence`
        (:`then_0`
          (set `TileActor.HorizontalIndex` (`self.HorizontalIndex`) _returnvalue_2))
        (:`then_1`
          (set `TileActor.VerticalIndex` (+ (`self.VerticalIndex`) 1) _returnvalue_2))
        (:`then_2`
          (bind _output_get (set `TileActor.MapData` (`self.MapData`) _returnvalue_2))
          (`MapManager.AddTileToGrid` _output_get _returnvalue_2))))))

(fn `Add Top (Plains)`
  (bind _returnvalue (`MapManager.GetTile` (`self.MapData`) (`self.HorizontalIndex`) (+ (`self.VerticalIndex`) 1)))
  (`/Engine/EditorBlueprintResources/StandardMacros.IsValid` _returnvalue
    (:`Is Not Valid`
      (bind _returnvalue_2 (`|SpawnActorFromClass` "/Game/Blueprints/MapTiles/PlainsTile.PlainsTile_C" (`KismetMathLibrary.MakeTransform` (+ (`self.K2_GetActorLocation`) (100.0 0.0 0.0))) "Undefined" "OverrideRootScale" null null))
      (`|ExecutionSequence`
        (:`then_0`
          (set `TileActor.HorizontalIndex` (`self.HorizontalIndex`) _returnvalue_2))
        (:`then_1`
          (set `TileActor.VerticalIndex` (+ (`self.VerticalIndex`) 1) _returnvalue_2))
        (:`then_2`
          (bind _output_get (set `TileActor.MapData` (`self.MapData`) _returnvalue_2))
          (`MapManager.AddTileToGrid` _output_get _returnvalue_2))))))

(fn `Add Top (Water)`
  (bind _returnvalue (`MapManager.GetTile` (`self.MapData`) (`self.HorizontalIndex`) (+ (`self.VerticalIndex`) 1)))
  (`/Engine/EditorBlueprintResources/StandardMacros.IsValid` _returnvalue
    (:`Is Not Valid`
      (bind _returnvalue_2 (`|SpawnActorFromClass` "/Game/Blueprints/MapTiles/WaterTile.WaterTile_C" (`KismetMathLibrary.MakeTransform` (+ (`self.K2_GetActorLocation`) (100.0 0.0 0.0))) "Undefined" "OverrideRootScale" null null))
      (`|ExecutionSequence`
        (:`then_0`
          (set `TileActor.HorizontalIndex` (`self.HorizontalIndex`) _returnvalue_2))
        (:`then_1`
          (set `TileActor.VerticalIndex` (+ (`self.VerticalIndex`) 1) _returnvalue_2))
        (:`then_2`
          (bind _output_get (set `TileActor.MapData` (`self.MapData`) _returnvalue_2))
          (`MapManager.AddTileToGrid` _output_get _returnvalue_2))))))

(fn `UserConstructionScript`)